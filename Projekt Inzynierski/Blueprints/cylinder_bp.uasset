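; Cylinder Blueprint that resets a cart-and-cylinder training run when the cylinder tilts too far or training completes.
; A delay on Tick throttles checks of roll and pitch against symmetric limits and the cart's TrainingComplete flag.
; On reset, it clears Start, teleports the cart to a fixed position, then moves the cylinder back and enables physics through delayed steps.
; It then sets Start again and clears TrainingComplete.
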(event `self.ReceiveTick`
  (params (DeltaSeconds :type "Float (single-precision)"))
  (`KismetSystemLibrary.Delay` 0.1)
  (if (or (> (`self.cylroll`) 30.0) (> (`self.cylpitch`) 30.0) (< (`self.cylroll`) -30.0) (< (`self.cylpitch`) -30.0) (`/Game/MindMaker/Examples/Assets/CartPole/cart_BP.TrainingComplete` (`self.cart`)))
    (set `self.start` false)
    (`SceneComponent.K2_SetWorldLocation` (`Actor.RootComponent` (`self.cart`)) (-10.0 -370.0 -40.0) false true)
    (`KismetSystemLibrary.Delay` 1.0)
    (`KismetSystemLibrary.MoveComponentTo` (`self.cylinder_bp`) (-10.0 -370.0 35.0) (struct) false false 0.0)
    (`KismetSystemLibrary.Delay` 1.0)
    (`PrimitiveComponent.SetSimulatePhysics` (`self.cylinder_bp`) true)
    (set `self.start` true)
    (set `/Game/MindMaker/Examples/Assets/CartPole/cart_BP.TrainingComplete` false (`self.cart`))))

(fn `UserConstructionScript`)