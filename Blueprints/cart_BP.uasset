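; MindMaker reinforcement learning agent: a cart cube that learns to steer past obstacle cubes, driven by an external learning engine over SocketIO.
; Each received action (three discrete choices) adjusts yaw and sets velocity, then five line-trace distances are sent back as observations with the reward.
; A low weighted distance sum counts as a crash, scoring Y progress, resetting the cart and randomizing obstacle X positions.
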(event `Delay for display`
  (bind _arrow (`self.Arrow`))
  (bind _cube (`self.Cube`))
  (bind _returnvalue (* (- (`self.ActionSelected`) 1.0) 10.0))
  ;[1 1 1] When displaying actions after training we divert from the normal recieve action function to this one so that a pause can be added as the agent moves between locations
  (`PrimitiveComponent.SetPhysicsLinearVelocity` _cube (* (`SceneComponent.GetForwardVector` _arrow) 300) false "None")
  (`SceneComponent.K2_AddWorldRotation` _arrow (`KismetMathLibrary.MakeRotator` 0.0 0.0 _returnvalue) false false)
  (`SceneComponent.K2_AddWorldRotation` _cube (`KismetMathLibrary.MakeRotator` 0.0 0.0 _returnvalue) false false)
  (`self.MakeObservations`)
  (`self.CheckReward`)
  (setmembers `/Game/MindMaker/Examples/Assets/CartPole/MindMakerCustomStructCartPole` :`StructRef` (`self.MindMakerStructure`) :`reward` (`self.Reward`) :`observations` (`self.Observations`) :`done` (`self.done`))
  (if (> (/ (+ (`self.Distance`) (/ (`self.Distance1`) 2.0) (/ (`self.Distance2`) 4.0) (/ (`self.Distance3`) 2.0) (/ (`self.Distance4`) 4.0)) 100.0) 2.0) :!label _label
    (`SocketIOClientComponent.Emit` (`self.SocketIOClient`) "sendobs" (`SIOJLibrary.Conv_StringToJsonValue` (`SIOJsonObject.EncodeJson` (`SIOJLibrary.StructToJsonObject` (`self.MindMakerStructure`)))) "/")
    (if (`self.TrainingComplete`)
      _)
    (else
      (`KismetSystemLibrary.PrintString` "waiting")
      (`KismetSystemLibrary.Delay` 0.1)
      (`self.MakeObservations`)
      (goto _label))))

(event `self.SocketIOClient.OnConnected`
  (params (SessionId :type String) (bIsReconnection :type Boolean))
  ;[1 1 1] Launch MindMaker
  ;;[1 1 1] If not using the mindmaker launcher plugin, manually launch mindmaker.exe before begining play. This is located in the MindMakerEngine directory within the projects Content folder. NOTE uses SocketIO to communicate with mindmaker.exe so your OS or antivirus may ask for user permission to access network.
  ;;[1 1 1] recieve messages from MindMaker
  (`SocketIOClientComponent.BindEventToFunction` (`self.SocketIOClient`) "messages" "Messages" null "/" "USE_DEFAULT") ; bind event to a bp function
  (`SocketIOClientComponent.BindEventToFunction` (`self.SocketIOClient`) "recaction" "ReceiveAction" null "/" "USE_DEFAULT") ; bind event to a bp function
  (`SocketIOClientComponent.BindEventToFunction` (`self.SocketIOClient`) "sendobs" "SendObservations" null "/" "USE_DEFAULT") ; bind event to a bp function
  (`SocketIOClientComponent.Connect` (`self.SocketIOClient`) "http://localhost:3000" "socket.io" null null)
  (`self.LaunchMindMaker` "NewEnumerator1" (`self.NumTrainingEpisodes`) (`self.NumEvalEpisodes`) false true "3" "low=0, high=1000, shape=(5,), dtype=np.float64" false true "ACKTR1000" false (`self.A2cParams`) (`self.AcerParams`) (`self.AcktrParams`) (`self.DqnParams`) (`self.Ppo2Params`) (`self.SacParams`) (`self.Td3Params`)))

(event `self.ReceiveBeginPlay`
  ;[1 1 1] Launch MindMaker
  ;;[1 1 1] To autolaunch the Mindmaker engine on event begin play, for instance in production use cases, requires the Mindmaker Launcher Plugin to be installed
  (`MindMakerBPLibrary.MindMakerWindows`)
  (`KismetSystemLibrary.PrintString` "MindMaker Launched")
  (`KismetSystemLibrary.PrintString` "Waiting for Connection from Learning Engine" true true (struct :`G` 0.66 :`B` 1.0 :`A` 1.0) 60.0))

(fn `CheckReward`
  (bind _cube1 (`self.cube1`))
  (bind _cube2 (`self.cube2`))
  (bind _cube (`self.Cube`))
  (bind _cube3 (`self.cube3`))
  (bind _cube4 (`self.cube4`))
  (bind _cube5 (`self.cube5`))
  (bind _cube6 (`self.cube6`))
  (bind _cube7 (`self.cube7`))
  (bind _cube8 (`self.cube8`))
  (bind (_returnvalue_x _returnvalue_y) (`KismetMathLibrary.BreakVector` (`SceneComponent.K2_GetComponentLocation` (`self.Cube`))))
  (bind (_returnvalue_x_2 _returnvalue_y_2 _returnvalue_z) (`KismetMathLibrary.BreakVector` (`self.K2_GetActorLocation` _cube8)))
  (bind (_returnvalue_x_3 _returnvalue_y_3 _returnvalue_z_2) (`KismetMathLibrary.BreakVector` (`self.K2_GetActorLocation` _cube1)))
  (bind (_returnvalue_x_4 _returnvalue_y_4 _returnvalue_z_3) (`KismetMathLibrary.BreakVector` (`self.K2_GetActorLocation` _cube2)))
  (bind (_returnvalue_x_5 _returnvalue_y_5 _returnvalue_z_4) (`KismetMathLibrary.BreakVector` (`self.K2_GetActorLocation` _cube3)))
  (bind (_returnvalue_x_6 _returnvalue_y_6 _returnvalue_z_5) (`KismetMathLibrary.BreakVector` (`self.K2_GetActorLocation` _cube4)))
  (bind (_returnvalue_x_7 _returnvalue_y_7 _returnvalue_z_6) (`KismetMathLibrary.BreakVector` (`self.K2_GetActorLocation` _cube5)))
  (bind (_returnvalue_x_8 _returnvalue_y_8 _returnvalue_z_7) (`KismetMathLibrary.BreakVector` (`self.K2_GetActorLocation` _cube6)))
  (bind (_returnvalue_x_9 _returnvalue_y_9 _returnvalue_z_8) (`KismetMathLibrary.BreakVector` (`self.K2_GetActorLocation` _cube7)))
  (if (> (/ (+ (`self.Distance`) (/ (`self.Distance1`) 2.0) (/ (`self.Distance2`) 4.0) (/ (`self.Distance3`) 2.0) (/ (`self.Distance4`) 4.0)) 100.0) 2.5)
    (set `self.Reward` 0.0)
    (else
      (bind _output_get (set `self.Reward` (- (/ _returnvalue_y 1500.0) 1.0)))
      (`SceneComponent.K2_SetWorldRotation` _cube (struct :`Yaw` 90.0) false false)
      (`SceneComponent.K2_SetWorldLocation` _cube (20.0 10.0 0.0) false true)
      (`PrimitiveComponent.SetPhysicsLinearVelocity` _cube (0.0 300.0 0.0) false "None")
      (`SceneComponent.K2_SetWorldRotation` (`self.Arrow`) (struct :`Yaw` 90.0) false false)
      (`self.K2_SetActorLocation` _cube1 (`KismetMathLibrary.MakeVector` (- (* (`KismetMathLibrary.RandomFloat`) 800.0) 400.0) _returnvalue_y_3 _returnvalue_z_2) false false)
      (`self.K2_SetActorLocation` _cube2 (`KismetMathLibrary.MakeVector` (- (* (`KismetMathLibrary.RandomFloat`) 800.0) 400.0) _returnvalue_y_4 _returnvalue_z_3) false false)
      (`self.K2_SetActorLocation` _cube3 (`KismetMathLibrary.MakeVector` (- (* (`KismetMathLibrary.RandomFloat`) 800.0) 400.0) _returnvalue_y_5 _returnvalue_z_4) false false)
      (`self.K2_SetActorLocation` _cube4 (`KismetMathLibrary.MakeVector` (- (* (`KismetMathLibrary.RandomFloat`) 800.0) 400.0) _returnvalue_y_6 _returnvalue_z_5) false false)
      (`self.K2_SetActorLocation` _cube5 (`KismetMathLibrary.MakeVector` (- (* (`KismetMathLibrary.RandomFloat`) 800.0) 400.0) _returnvalue_y_7 _returnvalue_z_6) false false)
      (`self.K2_SetActorLocation` _cube6 (`KismetMathLibrary.MakeVector` (- (* (`KismetMathLibrary.RandomFloat`) 800.0) 400.0) _returnvalue_y_8 _returnvalue_z_7) false false)
      (`self.K2_SetActorLocation` _cube7 (`KismetMathLibrary.MakeVector` (- (* (`KismetMathLibrary.RandomFloat`) 800.0) 400.0) _returnvalue_y_9 _returnvalue_z_8) false false)
      (`self.K2_SetActorLocation` _cube8 (`KismetMathLibrary.MakeVector` (- (* (`KismetMathLibrary.RandomFloat`) 800.0) 400.0) _returnvalue_y_2 _returnvalue_z) false false)
      (`KismetSystemLibrary.PrintString` (`KismetStringLibrary.Conv_DoubleToString` _output_get) true true (struct :`G` 0.66 :`B` 1.0 :`A` 1.0) 1.0))))

(fn `LaunchMindMaker`
  (params (`RL Algorithm` :type "/Game/MindMaker/Examples/Assets/CartPole/LearningAlgorithms Enum" :default "NewEnumerator3") (NumTrainEp :type Integer) (NumEvalEp :type Integer) (ContinousActionSpace :type Boolean) (`Discrete Action Space` :type Boolean) (`Action Space Shape` :type String) (`Observation Space Shape` :type String) (LoadPreTrainedModel :type Boolean) (SaveModelAfterTraining :type Boolean) (`Save/LoadModelName` :type String) (UseCustomParams :type Boolean) (A2cCustomParams :type "/Game/MindMaker/Examples/Assets/CartPole/A2cCustomParameters Structure") (AcerCustomParams :type "/Game/MindMaker/Examples/Assets/CartPole/AcerCustomParameters Structure") (AcktrCustomParams :type "/Game/MindMaker/Examples/Assets/CartPole/AcktrCustomParameters Structure") (DqnCustomParams :type "/Game/MindMaker/Examples/Assets/CartPole/DqnCustomParameters Structure") (Ppo2CustomParams :type "/Game/MindMaker/Examples/Assets/CartPole/PPO2CustomParameters Structure") (SacCustomParams :type "/Game/MindMaker/Examples/Assets/CartPole/SacCustomParameters Structure") (Td3CustomParams :type "/Game/MindMaker/Examples/Assets/CartPole/Td3CustomParameters Structure"))
  ;[1 1 1] Set members of our custom structure used for storing variables and pass them to neural network
  (setmembers `/Game/MindMaker/Examples/Assets/CartPole/MindMakerCustomStructCartPole` :`StructRef` (`self.MindMakerStructure`) :`reward` (`self.Reward`) :`observations` (`self.Observations`) :`trainepisodes` NumTrainEp :`evalepisodes` NumEvalEp :`maxactions` 0 :`loadmodel` (`KismetStringLibrary.Conv_BoolToString` LoadPreTrainedModel) :`savemodel` (`KismetStringLibrary.Conv_BoolToString` SaveModelAfterTraining) :`algselected` `RL Algorithm` :`customparams` (`KismetStringLibrary.Conv_BoolToString` UseCustomParams) :`modelname` `Save/LoadModelName` :`conactionspace` ContinousActionSpace :`minaction` (`self.MinActionVal`) :`maxaction` (`self.MaxActionVal`) :`done` false :`actionspace` `Action Space Shape` :`observationspace` `Observation Space Shape` :`disactionspace` `Discrete Action Space` :`a2cparams` A2cCustomParams :`acerparams` AcerCustomParams :`acktrparams` AcktrCustomParams :`dqnparams` DqnCustomParams :`ppo2params` Ppo2CustomParams :`sacparams` SacCustomParams :`td3params` Td3CustomParams)
  (`SocketIOClientComponent.Emit` (`self.SocketIOClient`) "launchmindmaker" (`SIOJLibrary.Conv_StringToJsonValue` (`SIOJsonObject.EncodeJson` (`SIOJLibrary.StructToJsonObject` (`self.MindMakerStructure`)))) "/"))

(fn `MakeObservations`
  (bind _returnvalue (`SceneComponent.K2_GetComponentLocation` (`self.Cube`)))
  ;[1 1 1] Enter observation values into array seperated by commas
  (bind _outhit (`KismetSystemLibrary.LineTraceSingle` _returnvalue (+ _returnvalue (* (`SceneComponent.GetForwardVector` (`self.Arrow`)) 1000)) "TraceTypeQuery1"))
  (bind (_bblockinghit _binitialoverlap _time _distance _location) (`GameplayStatics.BreakHitResult` _outhit))
  (`KismetSystemLibrary.DrawDebugLine` _returnvalue _location (struct :`R` 1.0 :`A` 1.0) 0.1 4.0)
  (bind _returnvalue_2 (`KismetMathLibrary.Vector_Distance` _returnvalue _location))
  (set `self.Distance` _returnvalue_2)
  (bind _outhit_2 (`KismetSystemLibrary.LineTraceSingle` _returnvalue (+ _returnvalue (* (`SceneComponent.GetForwardVector` (`self.Arrow1`)) 1000)) "TraceTypeQuery1"))
  (bind (_bblockinghit_2 _binitialoverlap_2 _time_2 _distance_2 _location_2) (`GameplayStatics.BreakHitResult` _outhit_2))
  (`KismetSystemLibrary.DrawDebugLine` _returnvalue _location_2 (struct :`R` 1.0 :`A` 1.0) 0.1 4.0)
  (bind _returnvalue_3 (`KismetMathLibrary.Vector_Distance` _location_2 _returnvalue))
  (set `self.Distance1` _returnvalue_3)
  (bind _outhit_3 (`KismetSystemLibrary.LineTraceSingle` _returnvalue (+ _returnvalue (* (`SceneComponent.GetForwardVector` (`self.Arrow2`)) 1000)) "TraceTypeQuery1"))
  (bind (_bblockinghit_3 _binitialoverlap_3 _time_3 _distance_3 _location_3) (`GameplayStatics.BreakHitResult` _outhit_3))
  (`KismetSystemLibrary.DrawDebugLine` _returnvalue _location_3 (struct :`R` 1.0 :`A` 1.0) 0.1 4.0)
  (bind _returnvalue_4 (`KismetMathLibrary.Vector_Distance` _location_3 _returnvalue))
  (set `self.Distance2` _returnvalue_4)
  (bind _outhit_4 (`KismetSystemLibrary.LineTraceSingle` _returnvalue (+ _returnvalue (* (`SceneComponent.GetForwardVector` (`self.Arrow3`)) 1000)) "TraceTypeQuery1"))
  (bind (_bblockinghit_4 _binitialoverlap_4 _time_4 _distance_4 _location_4) (`GameplayStatics.BreakHitResult` _outhit_4))
  (`KismetSystemLibrary.DrawDebugLine` _returnvalue _location_4 (struct :`R` 1.0 :`A` 1.0) 0.1 4.0)
  (bind _returnvalue_5 (`KismetMathLibrary.Vector_Distance` _location_4 _returnvalue))
  (set `self.Distance3` _returnvalue_5)
  (bind _outhit_5 (`KismetSystemLibrary.LineTraceSingle` _returnvalue (+ _returnvalue (* (`SceneComponent.GetForwardVector` (`self.Arrow4`)) 1000)) "TraceTypeQuery1"))
  (bind (_bblockinghit_5 _binitialoverlap_5 _time_5 _distance_5 _location_5) (`GameplayStatics.BreakHitResult` _outhit_5))
  (`KismetSystemLibrary.DrawDebugLine` _returnvalue _location_5 (struct :`R` 1.0 :`A` 1.0) 0.1 4.0)
  (bind _returnvalue_6 (`KismetMathLibrary.Vector_Distance` _location_5 _returnvalue))
  (set `self.Distance4` _returnvalue_6)
  (set `self.Observations` (`KismetStringLibrary.Concat_StrStr` "[" (`KismetStringLibrary.Conv_DoubleToString` _returnvalue_2) "," (`KismetStringLibrary.Conv_DoubleToString` _returnvalue_3) "," (`KismetStringLibrary.Conv_DoubleToString` _returnvalue_4) "," (`KismetStringLibrary.Conv_DoubleToString` _returnvalue_5) "," (`KismetStringLibrary.Conv_DoubleToString` _returnvalue_6) "]")))

(fn `Messages`
  (params (Message :type "SIOJsonValue Object Reference"))
  (bind _returnvalue (`SIOJsonValue.AsString` Message))
  ;[1 1 1] Display Messages From MindMaker.exe
  (`KismetSystemLibrary.PrintString` _returnvalue)
  (if (`KismetStringLibrary.EqualEqual_StrStr` _returnvalue "Training complete")
    (set `self.TrainingComplete` true)
    (elif (`KismetStringLibrary.EqualEqual_StrStr` _returnvalue "Evaluation Complete")
      (`KismetSystemLibrary.PrintString` "Quiting Game")
      (`KismetSystemLibrary.QuitGame` null "Quit")
      (else
        (`KismetSystemLibrary.PrintString` "Evaluating")))))

(fn `ReceiveAction`
  (params (Message :type "SIOJsonValue Object Reference"))
  (bind _returnvalue (`KismetStringLibrary.Conv_StringToDouble` (`KismetStringLibrary.Replace` (`KismetStringLibrary.Replace` (`|GetArrayItem` (`KismetStringLibrary.ParseIntoArray` (`SIOJsonValue.AsString` Message))) "[") "]")))
  ;[1 1 1] This recieves results from the neural network and updates the environment
  (set `self.ActionSelected` _returnvalue)
  (set `self.ActionRecieved` true)
  (`KismetSystemLibrary.PrintString` (`KismetStringLibrary.Concat_StrStr` "Predicted Action:" (`KismetStringLibrary.Conv_DoubleToString` _returnvalue)))
  (`self.Delay for display`))

(fn `UserConstructionScript`)